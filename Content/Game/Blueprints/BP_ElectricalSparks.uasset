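; BP_ElectricalSparks is an electrical hazard that damages and stuns the side-scroller player character on overlap.
; After applying damage, it polls with a short delay until the character lands, then forces a hop using a temporary damage jump velocity.
; It then slows walk speed to a random value and activates the character's spark particles until the stun duration ends, restoring the default speed.
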(event `self.ReceiveBeginPlay`
  (bind _asbp_side_scroller_character (cast `/Game/SideScrollerBP/Blueprints/BP_SideScrollerCharacter` (`GameplayStatics.GetPlayerCharacter` 0)))
  (set `self.BP Side Scroller Character` _asbp_side_scroller_character))

(event `self.CollisionComponent.OnComponentBeginOverlap`
  (params (OverlappedComponent :type "PrimitiveComponent Object Reference") (OtherActor :type "Actor Object Reference") (OtherComp :type "PrimitiveComponent Object Reference") (OtherBodyIndex :type Integer) (bFromSweep :type Boolean) (SweepResult :type "HitResult Structure (by ref)"))
  (bind _bp_side_scroller_character (`self.BP Side Scroller Character`))
  (bind _bp_side_scroller_character_2 (`self.BP Side Scroller Character`))
  (bind _charactermovement (`Character.CharacterMovement` _bp_side_scroller_character))
  (bind _charactermovement_2 (`Character.CharacterMovement` _bp_side_scroller_character))
  (if (== OtherActor _bp_side_scroller_character)
    (`GameplayStatics.ApplyDamage` _bp_side_scroller_character 15.0)
    (if (`NavMovementComponent.IsFalling` _charactermovement) :!label _label
      (`KismetSystemLibrary.Delay` 0.1)
      (goto _label)
      (else
        (set `CharacterMovementComponent.JumpZVelocity` (`/Game/SideScrollerBP/Blueprints/BP_SideScrollerCharacter.JumpHeightOnDamage` _bp_side_scroller_character) _charactermovement)
        (`Character.Jump` _bp_side_scroller_character)
        (`KismetSystemLibrary.Delay` 0.2)
        (set `CharacterMovementComponent.JumpZVelocity` (`/Game/SideScrollerBP/Blueprints/BP_SideScrollerCharacter.DefaultJump` (`self.BP Side Scroller Character`)) _charactermovement_2)
        (set `CharacterMovementComponent.MaxWalkSpeed` (`KismetMathLibrary.RandomFloatInRange` 200.0 350.0) _charactermovement_2)
        (`ActorComponent.Activate` (`/Game/SideScrollerBP/Blueprints/BP_SideScrollerCharacter.P_SparksBurst` (`self.BP Side Scroller Character`)) false)
        (`KismetSystemLibrary.Delay` (`self.StunDuration`))
        (set `CharacterMovementComponent.MaxWalkSpeed` (`/Game/SideScrollerBP/Blueprints/BP_SideScrollerCharacter.DefaultWalkSpeed` _bp_side_scroller_character_2) _charactermovement_2)
        (`ActorComponent.Deactivate` (`/Game/SideScrollerBP/Blueprints/BP_SideScrollerCharacter.P_SparksBurst` _bp_side_scroller_character_2))))))

(event `self.CollisionComponent.OnComponentEndOverlap`
  (params (OverlappedComponent :type "PrimitiveComponent Object Reference") (OtherActor :type "Actor Object Reference") (OtherComp :type "PrimitiveComponent Object Reference") (OtherBodyIndex :type Integer)))

(fn `UserConstructionScript`)